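; Blueprint function library that creates dynamic PBR material instances from a named color and material type.
; Select helpers find the name's index in library objects and read parallel arrays for color, metalness, specular and roughness.
; The Base variant writes these values to the shared Basic_PBR_MPC parameter collection, using the new instance only as world context.
; The Dynamic variant sets them as parameters on the instance itself.
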(fn `Create Base PBR Material Instance`
  (params (Mesh :type "Object Object Reference") (`Material to Instance` :type "MaterialInterface Object Reference") (`Color Name` :type "/Game/Blueprints/structs/player_PBR_colors_names Enum" :default "NewEnumerator0") (`Color Library` :type "/Game/Blueprints/structs/player_PBR_colors Structure") (`Material Type` :type "/Game/Blueprints/structs/PBR_material_names Enum" :default "NewEnumerator0") (`Material Library` :type "/Game/Blueprints/structs/PBR_materials Structure"))
  (returns (`Output Material Instance` :type "MaterialInterface Object Reference"))
  (bind _returnvalue (`KismetMaterialLibrary.CreateDynamicMaterialInstance` Mesh `Material to Instance`))
  (bind _color_output (`self.Select PBR Color` `Color Name` `Color Library`))
  (bind (_metalness_value _specular_value _roughness_value) (`self.Select PBR Material` `Material Type` `Material Library`))
  (`self.Set Base Material Values` _color_output _metalness_value _specular_value _roughness_value _returnvalue)
  (return _returnvalue))

(fn `Create Dynamic PBR Material Instance`
  (params (Mesh :type "Object Object Reference") (`Material to Instance` :type "Material Object Reference") (`Color Name` :type "/Game/Blueprints/structs/player_PBR_colors_names Enum" :default "NewEnumerator0") (`Color Library` :type "/Game/Blueprints/structs/player_PBR_colors Structure") (`Material Type` :type "/Game/Blueprints/structs/PBR_material_names Enum" :default "NewEnumerator0") (`Material Library` :type "/Game/Blueprints/structs/PBR_materials Structure"))
  (returns (`Output Material` :type "MaterialInstanceDynamic Object Reference"))
  (bind _returnvalue (`KismetMaterialLibrary.CreateDynamicMaterialInstance` Mesh `Material to Instance`))
  (bind _color_output (`self.Select PBR Color` `Color Name` `Color Library`))
  (bind (_metalness_value _specular_value _roughness_value) (`self.Select PBR Material` `Material Type` `Material Library`))
  (`self.Set PBR Material Parameters` _color_output _metalness_value _specular_value _roughness_value _returnvalue)
  (return _returnvalue))

(fn `Select PBR Color`
  (params (`Color Name` :type "/Game/Blueprints/structs/player_PBR_colors_names Enum" :default "NewEnumerator0") (`Set Library` :type "/Game/Blueprints/structs/player_PBR_colors Structure"))
  (returns (Color_output :type "Object.LinearColor Structure"))
  (bind (_pbr_names _pbr_values) (break `/Game/Blueprints/structs/player_PBR_colors` `Set Library`))
  (return (`KismetArrayLibrary.Array_Get` _pbr_values (`KismetArrayLibrary.Array_Find` _pbr_names `Color Name`))))

(fn `Select PBR Material`
  (params (`Material Type` :type "/Game/Blueprints/structs/PBR_material_names Enum" :default "NewEnumerator0") (`Set Library` :type "/Game/Blueprints/structs/PBR_materials Structure"))
  (returns (Metalness_value :type "Float (double-precision)") (Specular_value :type "Float (double-precision)") (Roughness_value :type "Float (double-precision)"))
  (bind (_pbr_material_type _pbr_metalness_value _pbr_specular_value _pbr_roughness_value) (break `/Game/Blueprints/structs/PBR_materials` `Set Library`))
  (bind _returnvalue (`KismetArrayLibrary.Array_Find` _pbr_material_type `Material Type`))
  (return (`KismetArrayLibrary.Array_Get` _pbr_metalness_value _returnvalue) (`KismetArrayLibrary.Array_Get` _pbr_specular_value _returnvalue) (`KismetArrayLibrary.Array_Get` _pbr_roughness_value _returnvalue)))

(fn `Set Base Material Values`
  (params (Base_Material_Color :type "Object.LinearColor Structure") (Base_Metalness :type "Float (double-precision)") (Base_Specular :type "Float (double-precision)") (Base_Roughness :type "Float (double-precision)") (Material_Instance :type "MaterialInstance Object Reference"))
  (`KismetMaterialLibrary.SetVectorParameterValue` Material_Instance "/Game/Materials/Basic_PBR_MPC.Basic_PBR_MPC" "Base_Material_Color" Base_Material_Color)
  (`KismetMaterialLibrary.SetScalarParameterValue` Material_Instance "/Game/Materials/Basic_PBR_MPC.Basic_PBR_MPC" "Base_Metalness" Base_Metalness)
  (`KismetMaterialLibrary.SetScalarParameterValue` Material_Instance "/Game/Materials/Basic_PBR_MPC.Basic_PBR_MPC" "Base_Specular" Base_Specular)
  (`KismetMaterialLibrary.SetScalarParameterValue` Material_Instance "/Game/Materials/Basic_PBR_MPC.Basic_PBR_MPC" "Base_Roughness" Base_Roughness))

(fn `Set PBR Material Parameters`
  (params (Color :type "Object.LinearColor Structure") (Metalness :type "Float (double-precision)") (Specular :type "Float (double-precision)") (Roughness :type "Float (double-precision)") (`Material Instance` :type "MaterialInstanceDynamic Object Reference"))
  (`MaterialInstanceDynamic.SetVectorParameterValue` `Material Instance` "Base_Color" Color)
  (`MaterialInstanceDynamic.SetScalarParameterValue` `Material Instance` "Metalness" Metalness)
  (`MaterialInstanceDynamic.SetScalarParameterValue` `Material Instance` "Specular" Specular)
  (`MaterialInstanceDynamic.SetScalarParameterValue` `Material Instance` "Roughness" Roughness))