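; IWorldClock is a Blueprint interface for querying an in-game world clock.
; It declares getters for current seconds, minutes, hours, day, month with its name, year and total days.
; Further getters expose the lengths of a minute, hour, day, week, month and year.
; It holds only signatures with default returns, leaving timekeeping to implementers.
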(fn `IF_GetDay`
  (returns (Days :type Integer))
  (return 0))

(fn `IF_GetDayLength`
  (returns (Length :type Integer))
  (return 0))

(fn `IF_GetDaysTotal`
  (returns (`Total Days` :type Integer))
  (return 0))

(fn `IF_GetHourLength`
  (returns (Length :type Integer))
  (return 0))

(fn `IF_GetHours`
  (returns (Hours :type Integer))
  (return 0))

(fn `IF_GetMinuteLength`
  (returns (Length :type Integer))
  (return 0))

(fn `IF_GetMinutes`
  (returns (Minutes :type Integer))
  (return 0))

(fn `IF_GetMonth`
  (returns (Month :type Integer) (`Month Name` :type String))
  (return 0 ""))

(fn `IF_GetMonthLength`
  (returns (Length :type Integer))
  (return 0))

(fn `IF_GetSeconds`
  (returns (Seconds :type Integer))
  (return 0))

(fn `IF_GetWeekLength`
  (returns (Length :type Integer))
  (return 0))

(fn `IF_GetYear`
  (returns (Year :type Integer))
  (return 0))

(fn `IF_GetYearLength`
  (returns (Length :type Integer))
  (return 0))