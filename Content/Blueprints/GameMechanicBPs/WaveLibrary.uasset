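; Blueprint function library that computes sine wave values from amplitude, frequency and time.
; It offers simple, phase-shifted and damped variants, all built on degree-based sine (Sind).
; The damped variant multiplies the sine by time times negated half-life, so its magnitude grows linearly rather than following the exponential decay its comment describes.
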(fn WaveMakeSimple
  (params (Amplitude :type Float%20%28single-precision%29) (Frequency :type Float%20%28single-precision%29) (Time :type Float%20%28single-precision%29))
  ;[1 1 1] Make Simple Wave: func(y)=A(sin(f*t))
  (return (* Amplitude (Math|Trig|Sin(Degrees) (* Frequency Time)))))

(fn WaveMakePhaseShifted
  (params (Amplitude :type Float%20%28single-precision%29) (Frequency :type Float%20%28single-precision%29) (Time :type Float%20%28single-precision%29) (PhaseShift :type Float%20%28single-precision%29))
  ;[1 1 1] Make Phase Shifted Wave: func(y)=A(sin(f*t + phase))
  (return (* Amplitude (Math|Trig|Sin(Degrees) (+ (* Frequency Time) PhaseShift)))))

(fn WaveMakeDamped
  (params (Amplitude :type Float%20%28single-precision%29) (Frequency :type Float%20%28single-precision%29) (Time :type Float%20%28single-precision%29) (Halflife :type Float%20%28single-precision%29))
  ;[1 1 1] Wave Make Damped: Creates a wave with a diminishing amplitude over time. [Y= Amplitude*exp(-K*X)*sin((2*pi*X/Wavelength)]
  (LocalVariables|SettempTime Time)
  (return (* Amplitude (Math|Trig|Sin(Degrees) (* Frequency (LocalVariables|GettempTime))) (* (LocalVariables|GettempTime) (* Halflife -1.0)))))