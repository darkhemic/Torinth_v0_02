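; Blueprint function library of per-field setters for the character data structs: vitals, identity info and personality.
; Each function takes a struct and a new value, then returns a rebuilt copy with that one field replaced and all others copied through.
; Vitals cover current and max HP, MP, fatigue and weight, while personality covers focus, perception, judging and dominant processes plus type.
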(fn `Char CVCurFatigue`
  (params (`Input Struct` :type "/Game/Blueprints/GameStructs/Stats/CharVitals Structure") (`New Value` :type Integer))
  (returns (`new Struct` :type "/Game/Blueprints/GameStructs/Stats/CharVitals Structure"))
  (bind (_curhp _maxhp _curmp _maxmp _curfatigue _maxfatigue _curweight _maxweight) (break `/Game/Blueprints/GameStructs/Stats/CharVitals` `Input Struct`))
  (return (make `/Game/Blueprints/GameStructs/Stats/CharVitals` _curhp _maxhp _curmp _maxmp `New Value` _maxfatigue _curweight _maxweight)))

(fn `Char CVCurHP`
  (params (`Input Struct` :type "/Game/Blueprints/GameStructs/Stats/CharVitals Structure") (`New Value` :type Integer))
  (returns (`new Struct` :type "/Game/Blueprints/GameStructs/Stats/CharVitals Structure"))
  (bind (_curhp _maxhp _curmp _maxmp _curfatigue _maxfatigue _curweight _maxweight) (break `/Game/Blueprints/GameStructs/Stats/CharVitals` `Input Struct`))
  (return (make `/Game/Blueprints/GameStructs/Stats/CharVitals` `New Value` _maxhp _curmp _maxmp _curfatigue _maxfatigue _curweight _maxweight)))

(fn `Char CVCurMP`
  (params (`Input Struct` :type "/Game/Blueprints/GameStructs/Stats/CharVitals Structure") (`New Value` :type Integer))
  (returns (`new Struct` :type "/Game/Blueprints/GameStructs/Stats/CharVitals Structure"))
  (bind (_curhp _maxhp _curmp _maxmp _curfatigue _maxfatigue _curweight _maxweight) (break `/Game/Blueprints/GameStructs/Stats/CharVitals` `Input Struct`))
  (return (make `/Game/Blueprints/GameStructs/Stats/CharVitals` _curhp _maxhp `New Value` _maxmp _curfatigue _maxfatigue _curweight _maxweight)))

(fn `Char CVCurWeight`
  (params (`Input Struct` :type "/Game/Blueprints/GameStructs/Stats/CharVitals Structure") (`New Value` :type Integer))
  (returns (`new Struct` :type "/Game/Blueprints/GameStructs/Stats/CharVitals Structure"))
  (bind (_curhp _maxhp _curmp _maxmp _curfatigue _maxfatigue _curweight _maxweight) (break `/Game/Blueprints/GameStructs/Stats/CharVitals` `Input Struct`))
  (return (make `/Game/Blueprints/GameStructs/Stats/CharVitals` _curhp _maxhp _curmp _maxmp _curfatigue _maxfatigue `New Value` _maxweight)))

(fn `Char CVMaxFatigue`
  (params (`Input Struct` :type "/Game/Blueprints/GameStructs/Stats/CharVitals Structure") (`New Value` :type Integer))
  (returns (`new Struct` :type "/Game/Blueprints/GameStructs/Stats/CharVitals Structure"))
  (bind (_curhp _maxhp _curmp _maxmp _curfatigue _maxfatigue _curweight _maxweight) (break `/Game/Blueprints/GameStructs/Stats/CharVitals` `Input Struct`))
  (return (make `/Game/Blueprints/GameStructs/Stats/CharVitals` _curhp _maxhp _curmp _maxmp _curfatigue `New Value` _curweight _maxweight)))

(fn `Char CVMaxMP`
  (params (`Input Struct` :type "/Game/Blueprints/GameStructs/Stats/CharVitals Structure") (`New Value` :type Integer))
  (returns (`new Struct` :type "/Game/Blueprints/GameStructs/Stats/CharVitals Structure"))
  (bind (_curhp _maxhp _curmp _maxmp _curfatigue _maxfatigue _curweight _maxweight) (break `/Game/Blueprints/GameStructs/Stats/CharVitals` `Input Struct`))
  (return (make `/Game/Blueprints/GameStructs/Stats/CharVitals` _curhp _maxhp _curmp `New Value` _curfatigue _maxfatigue _curweight _maxweight)))

(fn `Char CVMaxWeight`
  (params (`Input Struct` :type "/Game/Blueprints/GameStructs/Stats/CharVitals Structure") (`New Value` :type Integer))
  (returns (`new Struct` :type "/Game/Blueprints/GameStructs/Stats/CharVitals Structure"))
  (bind (_curhp _maxhp _curmp _maxmp _curfatigue _maxfatigue _curweight) (break `/Game/Blueprints/GameStructs/Stats/CharVitals` `Input Struct`))
  (return (make `/Game/Blueprints/GameStructs/Stats/CharVitals` _curhp _maxhp _curmp _maxmp _curfatigue _maxfatigue _curweight `New Value`)))

(fn `Char PSDominantProcess`
  (params (`Target Struct` :type "/Game/Blueprints/GameStructs/Personality/CharPersonality Structure") (`New Value` :type "Float (double-precision)"))
  (returns (Struct :type "/Game/Blueprints/GameStructs/Personality/CharPersonality Structure"))
  (bind (_focusdirection _perceptionprocess _judgingprocess _dominantprocess _personalitytype) (break `/Game/Blueprints/GameStructs/Personality/CharPersonality` `Target Struct`))
  (return (make `/Game/Blueprints/GameStructs/Personality/CharPersonality` _focusdirection _perceptionprocess _judgingprocess `New Value` _personalitytype)))

(fn `Char PSJudgingProcess`
  (params (`Target Struct` :type "/Game/Blueprints/GameStructs/Personality/CharPersonality Structure") (`New Value` :type "Float (double-precision)"))
  (returns (Struct :type "/Game/Blueprints/GameStructs/Personality/CharPersonality Structure"))
  (bind (_focusdirection _perceptionprocess _judgingprocess _dominantprocess _personalitytype) (break `/Game/Blueprints/GameStructs/Personality/CharPersonality` `Target Struct`))
  (return (make `/Game/Blueprints/GameStructs/Personality/CharPersonality` _focusdirection _perceptionprocess `New Value` _dominantprocess _personalitytype)))

(fn `Char PSPerceptionProcess`
  (params (`Target Struct` :type "/Game/Blueprints/GameStructs/Personality/CharPersonality Structure") (`New Value` :type "Float (double-precision)"))
  (returns (Struct :type "/Game/Blueprints/GameStructs/Personality/CharPersonality Structure"))
  (bind (_focusdirection _perceptionprocess _judgingprocess _dominantprocess _personalitytype) (break `/Game/Blueprints/GameStructs/Personality/CharPersonality` `Target Struct`))
  (return (make `/Game/Blueprints/GameStructs/Personality/CharPersonality` _focusdirection `New Value` _judgingprocess _dominantprocess _personalitytype)))

(fn `Char PSPersonalityType`
  (params (`Target Struct` :type "/Game/Blueprints/GameStructs/Personality/CharPersonality Structure") (`New Value` :type "/Game/Blueprints/GameInfo/Enums/MOBSpecific/EPersonalityTypes Enum" :default "NewEnumerator0"))
  (returns (Struct :type "/Game/Blueprints/GameStructs/Personality/CharPersonality Structure"))
  (bind (_focusdirection _perceptionprocess _judgingprocess _dominantprocess) (break `/Game/Blueprints/GameStructs/Personality/CharPersonality` `Target Struct`))
  (return (make `/Game/Blueprints/GameStructs/Personality/CharPersonality` _focusdirection _perceptionprocess _judgingprocess _dominantprocess `New Value`)))

(fn `CharCVMaxHP`
  (params (`Input Struct` :type "/Game/Blueprints/GameStructs/Stats/CharVitals Structure") (`New Value` :type Integer))
  (returns (`new Struct` :type "/Game/Blueprints/GameStructs/Stats/CharVitals Structure"))
  (bind (_curhp _maxhp _curmp _maxmp _curfatigue _maxfatigue _curweight _maxweight) (break `/Game/Blueprints/GameStructs/Stats/CharVitals` `Input Struct`))
  (return (make `/Game/Blueprints/GameStructs/Stats/CharVitals` _curhp `New Value` _curmp _maxmp _curfatigue _maxfatigue _curweight _maxweight)))

(fn `CharInfoAge`
  (params (`New Age` :type Integer) (`Target Struct` :type "/Game/Blueprints/GameStructs/Personality/CharInfo Structure"))
  (returns (`New Struct` :type "/Game/Blueprints/GameStructs/Personality/CharInfo Structure"))
  (bind (_givenname _surname _title _suffix _race _gender _citizenship _age _birthday _birthmonth _birthyear) (break `/Game/Blueprints/GameStructs/Personality/CharInfo` `Target Struct`))
  (return (make `/Game/Blueprints/GameStructs/Personality/CharInfo` _givenname _surname _title _suffix _race _gender _citizenship `New Age` _birthday 0 _birthyear)))

(fn `CharInfoBirthday`
  (params (`New Birthdate` :type Integer) (`Target Struct` :type "/Game/Blueprints/GameStructs/Personality/CharInfo Structure"))
  (returns (`New Struct` :type "/Game/Blueprints/GameStructs/Personality/CharInfo Structure"))
  (bind (_givenname _surname _title _suffix _race _gender _citizenship _age _birthday _birthmonth _birthyear) (break `/Game/Blueprints/GameStructs/Personality/CharInfo` `Target Struct`))
  (return (make `/Game/Blueprints/GameStructs/Personality/CharInfo` _givenname _surname _title _suffix _race _gender _citizenship _age `New Birthdate` 0 _birthyear)))

(fn `CharInfoBirthYear`
  (params (`New Birth Year` :type Integer) (`Target Struct` :type "/Game/Blueprints/GameStructs/Personality/CharInfo Structure"))
  (returns (`New Struct` :type "/Game/Blueprints/GameStructs/Personality/CharInfo Structure"))
  (bind (_givenname _surname _title _suffix _race _gender _citizenship _age _birthday) (break `/Game/Blueprints/GameStructs/Personality/CharInfo` `Target Struct`))
  (return (make `/Game/Blueprints/GameStructs/Personality/CharInfo` _givenname _surname _title _suffix _race _gender _citizenship _age _birthday 0 `New Birth Year`)))

(fn `CharInfoCitizenship`
  (params (`New Citizenship` :type "/Game/Blueprints/GameInfo/Enums/GenericInfo/EPlayerNations Enum" :default "NewEnumerator0") (`Target Struct` :type "/Game/Blueprints/GameStructs/Personality/CharInfo Structure"))
  (returns (`New Struct` :type "/Game/Blueprints/GameStructs/Personality/CharInfo Structure"))
  (bind (_givenname _surname _title _suffix _race _gender _citizenship _age _birthday _birthmonth _birthyear) (break `/Game/Blueprints/GameStructs/Personality/CharInfo` `Target Struct`))
  (return (make `/Game/Blueprints/GameStructs/Personality/CharInfo` _givenname _surname _title _suffix _race _gender `New Citizenship` _age _birthday 0 _birthyear)))

(fn `CharInfoGender`
  (params (`New Race` :type "/Game/Blueprints/GameInfo/Enums/MOBSpecific/EGenders Enum" :default "NewEnumerator0") (`Target Struct` :type "/Game/Blueprints/GameStructs/Personality/CharInfo Structure"))
  (returns (`New Struct` :type "/Game/Blueprints/GameStructs/Personality/CharInfo Structure"))
  (bind (_givenname _surname _title _suffix _race _gender _citizenship _age _birthday _birthmonth _birthyear) (break `/Game/Blueprints/GameStructs/Personality/CharInfo` `Target Struct`))
  (return (make `/Game/Blueprints/GameStructs/Personality/CharInfo` _givenname _surname _title _suffix _race `New Race` _citizenship _age _birthday 0 _birthyear)))

(fn `CharInfoName`
  (params (`New Name` :type String) (`Target Struct` :type "/Game/Blueprints/GameStructs/Personality/CharInfo Structure"))
  (returns (`New Struct` :type "/Game/Blueprints/GameStructs/Personality/CharInfo Structure"))
  (bind (_givenname _surname _title _suffix _race _gender _citizenship _age _birthday _birthmonth _birthyear) (break `/Game/Blueprints/GameStructs/Personality/CharInfo` `Target Struct`))
  (return (make `/Game/Blueprints/GameStructs/Personality/CharInfo` `New Name` _surname _title _suffix _race _gender _citizenship _age _birthday 0 _birthyear)))

(fn `CharInfoRace`
  (params (`New Race` :type "/Game/Blueprints/GameInfo/Enums/MOBSpecific/EPlayerRaces Enum" :default "NewEnumerator0") (`Target Struct` :type "/Game/Blueprints/GameStructs/Personality/CharInfo Structure"))
  (returns (`New Struct` :type "/Game/Blueprints/GameStructs/Personality/CharInfo Structure"))
  (bind (_givenname _surname _title _suffix _race _gender _citizenship _age _birthday _birthmonth _birthyear) (break `/Game/Blueprints/GameStructs/Personality/CharInfo` `Target Struct`))
  (return (make `/Game/Blueprints/GameStructs/Personality/CharInfo` _givenname _surname _title _suffix `New Race` _gender _citizenship _age _birthday 0 _birthyear)))

(fn `CharInfoSuffix`
  (params (`New Suffix` :type "/Game/Blueprints/GameInfo/Enums/MOBSpecific/EPlayerSuffix Enum" :default "NewEnumerator0") (`Target Struct` :type "/Game/Blueprints/GameStructs/Personality/CharInfo Structure"))
  (returns (`New Struct` :type "/Game/Blueprints/GameStructs/Personality/CharInfo Structure"))
  (bind (_givenname _surname _title _suffix _race _gender _citizenship _age _birthday _birthmonth _birthyear) (break `/Game/Blueprints/GameStructs/Personality/CharInfo` `Target Struct`))
  (return (make `/Game/Blueprints/GameStructs/Personality/CharInfo` _givenname _surname _title `New Suffix` _race _gender _citizenship _age _birthday 0 _birthyear)))

(fn `CharInfoSurname`
  (params (`New Name` :type String) (`Target Struct` :type "/Game/Blueprints/GameStructs/Personality/CharInfo Structure"))
  (returns (`New Struct` :type "/Game/Blueprints/GameStructs/Personality/CharInfo Structure"))
  (bind (_givenname _surname _title _suffix _race _gender _citizenship _age _birthday _birthmonth _birthyear) (break `/Game/Blueprints/GameStructs/Personality/CharInfo` `Target Struct`))
  (return (make `/Game/Blueprints/GameStructs/Personality/CharInfo` _givenname `New Name` _title _suffix _race _gender _citizenship _age _birthday 0 _birthyear)))

(fn `CharInfoTitle`
  (params (`New Title` :type "/Game/Blueprints/GameInfo/Enums/MOBSpecific/EPlayerTitles Enum" :default "NewEnumerator0") (`Target Struct` :type "/Game/Blueprints/GameStructs/Personality/CharInfo Structure"))
  (returns (`New Struct` :type "/Game/Blueprints/GameStructs/Personality/CharInfo Structure"))
  (bind (_givenname _surname _title _suffix _race _gender _citizenship _age _birthday _birthmonth _birthyear) (break `/Game/Blueprints/GameStructs/Personality/CharInfo` `Target Struct`))
  (return (make `/Game/Blueprints/GameStructs/Personality/CharInfo` _givenname _surname `New Title` _suffix _race _gender _citizenship _age _birthday 0 _birthyear)))

(fn `CharPSFocusDirection`
  (params (`Target Struct` :type "/Game/Blueprints/GameStructs/Personality/CharPersonality Structure") (`New Value` :type "Float (double-precision)"))
  (returns (Struct :type "/Game/Blueprints/GameStructs/Personality/CharPersonality Structure"))
  (bind (_focusdirection _perceptionprocess _judgingprocess _dominantprocess _personalitytype) (break `/Game/Blueprints/GameStructs/Personality/CharPersonality` `Target Struct`))
  (return (make `/Game/Blueprints/GameStructs/Personality/CharPersonality` `New Value` _perceptionprocess _judgingprocess _dominantprocess _personalitytype)))