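; Blueprint function library that derives max health, mana, fatigue and combat stats from a character's attributes via interface getters.
; Maximums multiply two scaled attributes; base combat stats divide three-attribute sums by an enum count, except magic attack, which multiplies.
; Calc wrappers await modifiers: magic defense calls the ranged base, and magic and ranged damage return zero.
; Also holds empty influence stubs, an offset-based stat-pairing helper and a debug logger.
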(fn CalcStatPrimeInfluence)

(fn CalcStatSecondaryInfluence)

(fn CalcStatPrimeOpposite)

(fn CalcStatSecondaryOpposite)

(fn PairInfluencesbyOrder
  (params (Baseline :type Integer) (OrderArray :type Array%20of%20EStats%20Enums) (OffsetIndex :type Byte) (OffsetArray :type Array%20of%20Bytes))
  ;[1 1 1] Initialize temp array and make sure it is clear
  (Utilities|Array|Clear (LocalVariables|GetInfArray))
  ;[1 1 1] Store the array length for later use.
  (LocalVariables|SetByte2 (Math|Conversions|ToByte(Integer) (Utilities|Array|Length OffsetArray)))
  ;[1 1 1] Loop through the offset array, and apply the offset at each element to the basline index
  (for _array_element OffsetArray
    ;;[1 1 1] Add offset to index
    (LocalVariables|SetByte1 (+ _array_element (Utilities|Array|Get(acopy) OrderArray Baseline)))
    (if (and (!= (LocalVariables|GetByte1) (LocalVariables|GetByte2)) (== (.Remainder (Math|Float|Division(WholeandRemainder) (Math|Conversions|ToFloat(Byte) (LocalVariables|GetByte1)) (Math|Conversions|ToFloat(Byte) (LocalVariables|GetByte2)))) 0.0))
      (LocalVariables|SetByte3 (Math|Conversions|ToByte(Integer) (Math|Float|Floor (.Remainder (Math|Float|Division(WholeandRemainder) (Math|Conversions|ToFloat(Byte) (LocalVariables|GetByte1)) (Math|Conversions|ToFloat(Byte) (LocalVariables|GetByte2)))))))
      (else
        (LocalVariables|SetByte3 0)))
    (Utilities|Array|Insert (LocalVariables|GetInfArray) (Utilities|Enum|ByteToEnumEStats (LocalVariables|GetByte3))))
  (return (LocalVariables|GetInfArray)))

(fn CalcMaxMana
  (params (Target :type Actor%20Object%20Reference))
  (LocalVariables|SetTargetActor Target)
  (bind _intelligence (Class|ICharStats|IFGetIntelligence(Message) (LocalVariables|GetTargetActor)))
  (LocalVariables|SetTInt _intelligence)
  (bind _wisdom (Class|ICharStats|IFGetWisdom(Message) (LocalVariables|GetTargetActor)))
  (LocalVariables|SetTWis _wisdom)
  (return (* (* (LocalVariables|GetTWis) 5) (* (LocalVariables|GetTInt) 5))))

(fn CalcMaxHealth
  (params (Target :type Actor%20Object%20Reference))
  (LocalVariables|SetTargetActor Target)
  (bind _strength (Class|ICharStats|IFGetStrength(Message) (LocalVariables|GetTargetActor)))
  (LocalVariables|SetTStrength _strength)
  (bind _constitution (Class|ICharStats|IFGetConstitution(Message) (LocalVariables|GetTargetActor)))
  (LocalVariables|SetTConstitution _constitution)
  (return (* (* (LocalVariables|GetTStrength) 5) (* (LocalVariables|GetTConstitution) 5))))

(fn CalcMaxFatigue
  (params (Target :type Actor%20Object%20Reference))
  (LocalVariables|SetTargetActor Target)
  (bind _wisdom (Class|ICharStats|IFGetWisdom(Message) (LocalVariables|GetTargetActor)))
  (LocalVariables|SetTWis _wisdom)
  (bind _constitution (Class|ICharStats|IFGetConstitution(Message) (LocalVariables|GetTargetActor)))
  (LocalVariables|SetTConstitution _constitution)
  (return (* (* (LocalVariables|GetTWis) 5) (* (LocalVariables|GetTConstitution) 5))))

(fn CalcBasePhysAttack
  (params (Target :type Actor%20Object%20Reference))
  (LocalVariables|SetCSBPA_ARef Target)
  (bind _strength (Class|ICharStats|IFGetStrength(Message) (LocalVariables|GetCSBPA_ARef)))
  (LocalVariables|SetTStr _strength)
  (bind _dexterity (Class|ICharStats|IFGetDexterity(Message) (LocalVariables|GetCSBPA_ARef)))
  (LocalVariables|SetTDex _dexterity)
  (bind _perception (Class|ICharStats|IFGetPerception(Message) (LocalVariables|GetCSBPA_ARef)))
  (LocalVariables|SetTper _perception)
  (return (Math|Conversions|ToFloat(Integer) (/ (+ (LocalVariables|GetTStr) (LocalVariables|GetTDex) (LocalVariables|GetTper)) (|GetNumEnumEntries)))))

(fn CalcBasePhysDefense
  (params (Target :type Actor%20Object%20Reference))
  (LocalVariables|SetCSBPD_ARef Target)
  (bind _agility (Class|ICharStats|IFGetAgility(Message) (LocalVariables|GetCSBPD_ARef)))
  (LocalVariables|SetCSBPD_Agi _agility)
  (bind _constitution (Class|ICharStats|IFGetConstitution(Message) (LocalVariables|GetCSBPD_ARef)))
  (LocalVariables|SetCSBPD_Con _constitution)
  (bind _perception (Class|ICharStats|IFGetPerception(Message) (LocalVariables|GetCSBPD_ARef)))
  (LocalVariables|SetCSBPD_Per _perception)
  (return (Math|Conversions|ToFloat(Integer) (/ (+ (LocalVariables|GetCSBPD_Agi) (LocalVariables|GetCSBPD_Con) (LocalVariables|GetCSBPD_Per)) (|GetNumEnumEntries)))))

(fn CalcBasePhysDamage
  (params (Target :type Actor%20Object%20Reference))
  (LocalVariables|SetCSCBPD_ARef Target)
  (bind _strength (Class|ICharStats|IFGetStrength(Message) (LocalVariables|GetCSCBPD_ARef)))
  (LocalVariables|SetCSCBPD_Str _strength)
  (bind _perception (Class|ICharStats|IFGetPerception(Message) (LocalVariables|GetCSCBPD_ARef)))
  (LocalVariables|SetCSCBPD_Per _perception)
  (bind _dexterity (Class|ICharStats|IFGetDexterity(Message) (LocalVariables|GetCSCBPD_ARef)))
  (LocalVariables|SetCSCBPD_Dex _dexterity)
  (return (Math|Conversions|ToFloat(Integer) (/ (+ (LocalVariables|GetCSCBPD_Str) (LocalVariables|GetCSCBPD_Per) (LocalVariables|GetCSCBPD_Dex)) (|GetNumEnumEntries)))))

(fn CalcPhysDamage
  (params (Target :type Actor%20Object%20Reference))
  (LocalVariables|SetCSCPDa_Aref Target)
  (bind _base_phys_damage (FunctionLibraries|CombatStats|Damage|CalcBasePhysDamage (LocalVariables|GetCSCPDa_Aref)))
  (return _base_phys_damage))

(fn CalcPhysAttack
  (params (Target :type Actor%20Object%20Reference))
  (LocalVariables|SetCSPA_Aref Target)
  ;[1 1 1] Need to insert node for mods here.
  (bind _base_phys_attack (FunctionLibraries|CombatStats|Attack|CalcBasePhysAttack (LocalVariables|GetCSPA_Aref)))
  (return _base_phys_attack))

(fn CalcPhysDefense
  (params (Target :type Actor%20Object%20Reference))
  (LocalVariables|SetCSCPD_ARef Target)
  ;[1 1 1] Add Modifiers
  (bind _base_phys_defense (FunctionLibraries|CombatStats|Defense|CalcBasePhysDefense (LocalVariables|GetCSCPD_ARef)))
  (return _base_phys_defense))

(fn CalcMagAttack
  (params (Target :type Actor%20Object%20Reference))
  (LocalVariables|SetCSCMA_Aref Target)
  ;[1 1 1] Need to add in modifiers
  (bind _base_phys_attack (FunctionLibraries|CombatStats|Attack|CalcBaseMagAttack (LocalVariables|GetCSCMA_Aref)))
  (return _base_phys_attack))

(fn CalcBaseMagAttack
  (params (Target :type Actor%20Object%20Reference))
  (LocalVariables|SetCSBMA_ARef Target)
  (bind _intelligence (Class|ICharStats|IFGetIntelligence(Message) (LocalVariables|GetCSBMA_ARef)))
  (LocalVariables|SetCSBMA_Int _intelligence)
  (bind _wisdom (Class|ICharStats|IFGetWisdom(Message) (LocalVariables|GetCSBMA_ARef)))
  (LocalVariables|SetCSBMA_Wis _wisdom)
  (bind _charisma (Class|ICharStats|IFGetCharisma(Message) (LocalVariables|GetCSBMA_ARef)))
  (LocalVariables|SetCSBMA_Cha _charisma)
  (return (Math|Conversions|ToFloat(Integer) (* (+ (LocalVariables|GetCSBMA_Int) (LocalVariables|GetCSBMA_Wis) (LocalVariables|GetCSBMA_Cha)) (|GetNumEnumEntries)))))

(fn CalcMagDefense
  (params (Target :type Actor%20Object%20Reference))
  (LocalVariables|SetCSCMD_ARef Target)
  ;[1 1 1] Add Modifiers
  (bind _phys_defense (FunctionLibraries|CombatStats|Defense|CalcBaseRangeDefense (LocalVariables|GetCSCMD_ARef)))
  (return _phys_defense))

(fn CalcBaseMagDefense
  (params (Target :type Actor%20Object%20Reference))
  (LocalVariables|SetCSBMD_Aref Target)
  (bind _wisdom (Class|ICharStats|IFGetWisdom(Message) (LocalVariables|GetCSBMD_Aref)))
  (LocalVariables|SetCSBMD_Wis _wisdom)
  (bind _charisma (Class|ICharStats|IFGetCharisma(Message) (LocalVariables|GetCSBMD_Aref)))
  (LocalVariables|SetCSCBMD_Cha _charisma)
  (bind _perception (Class|ICharStats|IFGetPerception(Message) (LocalVariables|GetCSBMD_Aref)))
  (LocalVariables|SetCSBMD_Cha _perception)
  (return (Math|Conversions|ToFloat(Integer) (/ (+ (LocalVariables|GetCSBMD_Wis) (LocalVariables|GetCSCBMD_Cha) (LocalVariables|GetCSBMD_Cha)) (|GetNumEnumEntries)))))

(fn CalcRangeAttack
  (params (Target :type Actor%20Object%20Reference))
  (LocalVariables|SetCSCRA_Aref Target)
  ;[1 1 1] Need to add in Modifiers
  (bind _phys_attack (FunctionLibraries|CombatStats|Attack|CalcBaseRangeAttack (LocalVariables|GetCSCRA_Aref)))
  (return _phys_attack))

(fn CalcBaseRangeAttack
  (params (Target :type Actor%20Object%20Reference))
  (LocalVariables|SetCSMRA_Aref Target)
  (bind _perception (Class|ICharStats|IFGetPerception(Message) (LocalVariables|GetCSMRA_Aref)))
  (LocalVariables|SetCSRMA_Per _perception)
  (bind _dexterity (Class|ICharStats|IFGetDexterity(Message) (LocalVariables|GetCSMRA_Aref)))
  (LocalVariables|SetCSRMA_Dex _dexterity)
  (bind _wisdom (Class|ICharStats|IFGetWisdom(Message) (LocalVariables|GetCSMRA_Aref)))
  (LocalVariables|SetCSRMA_Wis _wisdom)
  (return (Math|Conversions|ToFloat(Integer) (/ (+ (LocalVariables|GetCSRMA_Per) (LocalVariables|GetCSRMA_Dex) (LocalVariables|GetCSRMA_Wis)) (|GetNumEnumEntries)))))

(fn CalcBaseRangeDefense
  (params (Target :type Actor%20Object%20Reference))
  (LocalVariables|SetCSBRD_Aref Target)
  (bind _agility (Class|ICharStats|IFGetAgility(Message) (LocalVariables|GetCSBRD_Aref)))
  (LocalVariables|SetCSBRD_AGI _agility)
  (bind _constitution (Class|ICharStats|IFGetConstitution(Message) (LocalVariables|GetCSBRD_Aref)))
  (LocalVariables|SetCSBRD_Con _constitution)
  (bind _perception (Class|ICharStats|IFGetPerception(Message) (LocalVariables|GetCSBRD_Aref)))
  (LocalVariables|SetCSBRD_Per _perception)
  (return (Math|Conversions|ToFloat(Integer) (/ (+ (LocalVariables|GetCSBRD_AGI) (LocalVariables|GetCSBRD_Con) (LocalVariables|GetCSBRD_Per)) (|GetNumEnumEntries)))))

(fn CalcRangeDefense
  (params (Target :type Actor%20Object%20Reference))
  (LocalVariables|SetCSCRD_Aref Target)
  (bind _phys_defense (FunctionLibraries|CombatStats|Defense|CalcBaseRangeDefense (LocalVariables|GetCSCRD_Aref)))
  (return _phys_defense))

(fn CalcMagDamage
  (params (Target :type Actor%20Object%20Reference))
  (return 0.0))

(fn CalcRangeDamage
  (params (Target :type Actor%20Object%20Reference))
  (return 0.0))

(fn CalcBaseMagDamage
  (params (Target :type Actor%20Object%20Reference))
  (LocalVariables|SetCSCBMD_ARef Target)
  (bind _intelligence (Class|ICharStats|IFGetIntelligence(Message) (LocalVariables|GetCSCBMD_ARef)))
  (LocalVariables|SetCSCBMD_Int _intelligence)
  (bind _perception (Class|ICharStats|IFGetPerception(Message) (LocalVariables|GetCSCBMD_ARef)))
  (LocalVariables|SetCSCBMD_Per _perception)
  (bind _wisdom (Class|ICharStats|IFGetWisdom(Message) (LocalVariables|GetCSCBMD_ARef)))
  (LocalVariables|SetCSCBMD_Wis _wisdom)
  (return (Math|Conversions|ToFloat(Integer) (/ (+ (LocalVariables|GetCSCBMD_Int) (LocalVariables|GetCSCBMD_Wis) (LocalVariables|GetCSCBMD_Per)) (|GetNumEnumEntries)))))

(fn CalcBaseRangeDamage
  (params (Target :type Actor%20Object%20Reference))
  (LocalVariables|SetCSCBPD_ARef Target)
  (bind _strength (Class|ICharStats|IFGetStrength(Message) (LocalVariables|GetCSCBPD_ARef)))
  (LocalVariables|SetCSCBRD_Str _strength)
  (bind _intelligence (Class|ICharStats|IFGetIntelligence(Message) (LocalVariables|GetCSCBPD_ARef)))
  (LocalVariables|SetCSCBRD_Int _intelligence)
  (bind _dexterity (Class|ICharStats|IFGetDexterity(Message) (LocalVariables|GetCSCBPD_ARef)))
  (LocalVariables|SetCSCBRD_Dex _dexterity)
  (return (Math|Conversions|ToFloat(Integer) (/ (+ (LocalVariables|GetCSCBRD_Str) (LocalVariables|GetCSCBRD_Dex) (LocalVariables|GetCSCBRD_Int)) (|GetNumEnumEntries)))))

(fn CheckDebugandLog
  (params (Skill/Stat%20Name :type String) (Function%20Name :type String) (Success%20Message :type String) (Failure%20Message :type String) (Character%20Ref :type Player%20Controller%20Object%20Reference) (Success :type Boolean))
  (LocalVariables|SetSucceeded Success)
  ;[1 1 1] Check for Debug Logging
  (bind _asdefault_gm (Utilities|Casting|CastToDefaultGM (Game|GetGameMode))
    (:then
      (if (Variables|/Game/Blueprints/GameMechanicBPs/DefaultGM.DefaultGM_C|GetDebugMode _asdefault_gm)
        ;[1 1 1] Log completion success or failure if debug is true.
        (if (LocalVariables|GetSucceeded)
          (Class|VisualLoggerKismetLibrary|LogText (Utilities|String|Append Skill/Stat%20Name ": ") "Blueprint Log")
          (else
            (Class|VisualLoggerKismetLibrary|LogText (Utilities|String|Append (Utilities|String|Append (Utilities|String|Append Skill/Stat%20Name ": .") Function%20Name) Failure%20Message) "Blueprint Log")))
        (return (LocalVariables|GetSucceeded))))
    (:CastFailed
      ;[1 1 1] Log failure to cast to default GM
      (Class|VisualLoggerKismetLibrary|LogText "Cast to DefaultGM from \"Root_CharStat>Set Base Control\" failed." "Blueprint Log")
      (return (LocalVariables|GetSucceeded)))))