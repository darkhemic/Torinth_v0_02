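; ICharInfo is a Blueprint interface for reading and editing a character's identity information.
; It declares modifier functions for name parts, title, race, gender, citizenship, age and birth day, each taking a new value and a target struct and returning a boolean.
; GetCharInfoStruct exposes the character info struct, and implementing classes supply all the logic.
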(fn `GetCharInfoStruct`
  (returns (`Character Info` :type "/Game/Blueprints/GameStructs/Personality/CharInfo Structure"))
  (return))

(fn `modify Age`
  (params (`New Age` :type Integer) (`Target Struct` :type "/Game/Blueprints/GameStructs/Personality/CharInfo Structure"))
  (returns (Return :type Boolean))
  (return false))

(fn `Modify Birth Day`
  (params (`New Day` :type Integer) (`Target Struct` :type "/Game/Blueprints/GameStructs/Personality/CharInfo Structure"))
  (returns (Return :type Boolean))
  (return false))

(fn `Modify Citizenship`
  (params (`New Citizenship` :type "/Game/Blueprints/GameInfo/Enums/GenericInfo/EPlayerNations Enum") (`Target Struct` :type "/Game/Blueprints/GameStructs/Personality/CharInfo Structure"))
  (returns (Return :type Boolean))
  (return false))

(fn `Modify Gender`
  (params (Gender :type "/Game/Blueprints/GameInfo/Enums/MOBSpecific/EGenders Enum") (`Target Struct` :type "/Game/Blueprints/GameStructs/Personality/CharInfo Structure"))
  (returns (Return :type Boolean))
  (return false))

(fn `Modify Given Name`
  (params (Name :type String) (`Target Struct` :type "/Game/Blueprints/GameStructs/Personality/CharInfo Structure"))
  (returns (Return :type Boolean))
  (return false))

(fn `Modify Race`
  (params (`New Race` :type "/Game/Blueprints/GameInfo/Enums/MOBSpecific/EPlayerRaces Enum") (`Target Struct` :type "/Game/Blueprints/GameStructs/Personality/CharInfo Structure"))
  (returns (Return :type Boolean))
  (return false))

(fn `Modify Suffix`
  (params (`New Suffix` :type "/Game/Blueprints/GameInfo/Enums/MOBSpecific/EPlayerSuffix Enum") (`Target Struct` :type "/Game/Blueprints/GameStructs/Personality/CharInfo Structure"))
  (returns (Return :type Boolean))
  (return false))

(fn `Modify Surname`
  (params (Surname :type String) (`Target Struct` :type "/Game/Blueprints/GameStructs/Personality/CharInfo Structure"))
  (returns (Return :type Boolean))
  (return false))

(fn `Modify Title`
  (params (NewTitle :type "/Game/Blueprints/GameInfo/Enums/MOBSpecific/EPlayerTitles Enum") (`Target Struct` :type "/Game/Blueprints/GameStructs/Personality/CharInfo Structure"))
  (returns (Return :type Boolean))
  (return false))