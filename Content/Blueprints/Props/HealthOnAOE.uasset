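; HealthOnAOE is a prop that periodically heals the player through an area check.
; A looping one-second timer scans every Character and, for each within a fixed radius of the prop, sends ModifyCharHealth to player pawn 0, not to that Character, so heals stack per Character in range.
; Cursor-over events only print placeholder text, and GetContextMenu returns the prop's ContextMenu.
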(event `self.ReceiveBeginPlay`
  (`KismetSystemLibrary.K2_SetTimerDelegate` (delegate `Heal Player`) 1.0 true))

(event `Heal Player`
  (bind _outactors (`GameplayStatics.GetAllActorsOfClass` "/Script/Engine.Character"))
  (for _array_element _outactors
    (if (<= (`KismetMathLibrary.VSize` (- (`self.K2_GetActorLocation` _array_element) (`self.K2_GetActorLocation`))) 250.0)
      (message `/Game/Blueprints/Interfaces/CharacterInterfaces/ICharVitals.ModifyCharHealth` (`GameplayStatics.GetPlayerPawn` 0) 10.0))))

(event `self.ReceiveActorBeginCursorOver`
  ;[1 1 1] Place Holder for MouseOver Events
  (`KismetSystemLibrary.PrintString` "Mouse Over!!"))

(event `self.ReceiveActorEndCursorOver`
  ;[1 1 1] Place Holder for MouseOver Events
  (`KismetSystemLibrary.PrintString` "End Mouse Over!!"))

(fn `GetContextMenu`
  (returns (ContextMenu :type "Array of /Game/Blueprints/GameInfo/Enums/MenuItems/EContextMenu Enum"))
  (return (`self.context menu`)))

(fn `UserConstructionScript`)